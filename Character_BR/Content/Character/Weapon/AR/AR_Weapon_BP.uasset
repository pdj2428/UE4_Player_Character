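; Assault rifle weapon Blueprint that sets its weapon kind on BeginPlay and adds rifle-specific shell ejection and reload visuals.
; The casing drop event spawns a casing with random pitch at the bullet spawn component, enables physics, and applies a randomized backward, leftward, slightly downward velocity impulse scaled around the passed value.
; The reload event hides the magazine by swapping its "Clip" material slot to an invisible material, restoring it when reloading ends.
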(event `self.ReceiveBeginPlay`
  (set `self.WeaponKind` "EWK_AssaultRifle"))

(event `self.ReceiveTick`
  (params (DeltaSeconds :type "Float (single-precision)"))
  (`parent.ReceiveTick` DeltaSeconds))

(event `EventBulletCashingDrop`
  (params (Value :type "Float (double-precision)"))
  (bind (_negative _positive) (`/Game/Character/Function/MathLibrary.GettingNegativeAndPositive` 10.0))
  (bind (_lower _upper) (`/Game/Character/Function/MathLibrary.LowerAndUpper` Value 50.0))
  (bind _returnvalue (`|SpawnActorFromClass` "/Game/Character/Weapon/BulletCasingActor.BulletCasingActor_C" (`KismetMathLibrary.MakeTransform` (0.0 0.0 0.0) (`KismetMathLibrary.MakeRotator` 0.0 (`KismetMathLibrary.RandomFloatInRange` _negative _positive))) "Undefined" "OverrideRootScale" null null))
  (`self.K2_AttachToComponent` _returnvalue (`self.SpawnBulletLocation`) "None" "KeepRelative" "KeepRelative" "KeepRelative" true)
  (bind _staticmesh (`/Game/Character/Weapon/BulletCasingActor.StaticMesh` _returnvalue))
  (`PrimitiveComponent.SetSimulatePhysics` _staticmesh true)
  (bind (_returnvalue_x _returnvalue_y _returnvalue_z) (`KismetMathLibrary.BreakVector` (+ (* (`self.GetActorForwardVector` _returnvalue) (* (`KismetMathLibrary.RandomFloatInRange` _lower _upper) -1.0)) (* (`self.GetActorRightVector` _returnvalue) (* (`KismetMathLibrary.RandomFloatInRange` _lower _upper) -1.0)))))
  (`PrimitiveComponent.AddImpulse` _staticmesh (`KismetMathLibrary.MakeVector` _returnvalue_x _returnvalue_y (- _returnvalue_z (`KismetMathLibrary.RandomFloatInRange` 0.0 50.0))) "None" true))

(event `ReloadClipMaterial`
  (params (IsReloading :type Boolean))
  (`PrimitiveComponent.SetMaterialByName` (`self.SkeletalMesh`) "Clip" (select `bool` IsReloading :`false` "/Game/Character/MilitaryWeapDark/Weapons/Materials/M_AssaultRifle_01.M_AssaultRifle_01" :`true` "/Game/Character/Weapon/Invisible_Mat.Invisible_Mat" :!type "MaterialInterface Object Reference")))

(fn `UserConstructionScript`
  (`parent.UserConstructionScript`))